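; PlanetObject_BP is a physics object that is pulled toward the planet in PlanetPawn_BP.
; On BeginPlay it caches the player's PlanetPawn and sets that planet as the second component of its PhysicsConstraint.
; Each Tick it applies a force toward the planet's center, scaled by object mass times pawn Gravity.
; The force is applied as an acceleration change despite that mass factor, and the BreakConstraint call is never triggered.
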(event `self.ReceiveBeginPlay`
  (`self.SetPlanetPawn`)
  (bind _returnvalue (`GameplayStatics.GetActorOfClass` "/Game/Blueprints/PlanetPawn_BP.PlanetPawn_BP_C"))
  (`PhysicsConstraintComponent.SetConstrainedComponents` (`self.PhysicsConstraint`) null "None" (`/Game/Blueprints/PlanetPawn_BP.Planet` _returnvalue) "None"))

(event `self.ReceiveTick`
  (params (DeltaSeconds :type "Float (single-precision)"))
  (`self.AddGravityForce`))

(fn `AddGravityForce`
  (bind _weight (`self.GetWeight`))
  (bind _velocitytoplanet (`self.GetVelocityToPlanet`))
  (`PrimitiveComponent.AddForce` (`self.Object`) (* (`KismetMathLibrary.Normal` _velocitytoplanet) _weight) "None" true))

(fn `GetVelocityToPlanet`
  (returns (VelocityToPlanet :type "Vector Structure"))
  (return (- (`SceneComponent.K2_GetComponentLocation` (`/Game/Blueprints/PlanetPawn_BP.Planet` (`self.PlanetPawn`))) (`SceneComponent.K2_GetComponentLocation` (`self.Object`)))))

(fn `GetWeight`
  (returns (Weight :type "Float (double-precision)"))
  (return (* (`PrimitiveComponent.GetMass` (`self.Object`)) (`/Game/Blueprints/PlanetPawn_BP.Gravity` (`self.PlanetPawn`)))))

(fn `SetPlanetPawn`
  (bind _asplanet_pawn_bp (cast `/Game/Blueprints/PlanetPawn_BP` (`GameplayStatics.GetPlayerPawn` 0)))
  (set `self.PlanetPawn` _asplanet_pawn_bp))

(fn `UserConstructionScript`)