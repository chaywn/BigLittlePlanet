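; Player controller that turns Enhanced Input into planet rotation, puppet jump, grip/release and level restart.
; On BeginPlay it adds the mapping context and caches the PlanetPawn_BP found in the level.
; Actions broadcast through event dispatchers, with jump and grip gated by the pawn's Puppet state: ground contact, current grip and object detection.
; Planet rotation is roll-only, and reset reopens the current level by name.
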(event `self.ReceiveBeginPlay`
  (`self.SetupInput`)
  (`self.SetPlanetPawn`))

(event `EnhancedInput|/Game/Input/IA_ResetLevel`
  (params (ActionValue :type Boolean) (ElapsedSeconds :type "Float (double-precision)") (TriggeredSeconds :type "Float (double-precision)") (InputAction :type "InputAction Object Reference" :default "/Game/Input/IA_ResetLevel.IA_ResetLevel"))
  (:`Triggered`
    (bind _returnvalue (`GameplayStatics.GetCurrentLevelName` true))
    (`GameplayStatics.OpenLevel` (`KismetStringLibrary.Conv_StringToName` _returnvalue))))

(event `EnhancedInput|/Game/Input/IA_RotatePlanet`
  (params (ActionValue :type "Vector2D Structure") (ElapsedSeconds :type "Float (double-precision)") (TriggeredSeconds :type "Float (double-precision)") (InputAction :type "InputAction Object Reference" :default "/Game/Input/IA_RotatePlanet.IA_RotatePlanet"))
  (:`Triggered`
    (`self.OnPlanetRotate` (`KismetMathLibrary.MakeRotator` ActionValue_X))))

(event `EnhancedInput|/Game/Input/IA_PuppetJump`
  (params (ActionValue :type Boolean) (ElapsedSeconds :type "Float (double-precision)") (TriggeredSeconds :type "Float (double-precision)") (InputAction :type "InputAction Object Reference" :default "/Game/Input/IA_PuppetJump.IA_PuppetJump"))
  (:`Triggered`
    (bind _onground (`self.PuppetOnGround`))
    (if _onground
      (`self.OnPuppetJump`))))

(event `EnhancedInput|/Game/Input/IA_GripObject`
  (params (ActionValue :type Boolean) (ElapsedSeconds :type "Float (double-precision)") (TriggeredSeconds :type "Float (double-precision)") (InputAction :type "InputAction Object Reference" :default "/Game/Input/IA_GripObject.IA_GripObject"))
  (:`Triggered`
    (bind _isgripping (`self.PuppetIsGripping`))
    (if _isgripping
      (`self.OnRelease`)
      (else
        (bind _isdetected (`/Game/Blueprints/Puppet_BP.DetectObject` (`/Game/Blueprints/PlanetPawn_BP.Puppet` (`self.PlanetPawn`))))
        (if _isdetected
          (`self.OnGrip`))))))

(fn `PuppetIsGripping`
  (returns (IsGripping :type Boolean))
  (return (`/Game/Blueprints/Puppet_BP.IsGripping` (`/Game/Blueprints/PlanetPawn_BP.Puppet` (`self.PlanetPawn`)))))

(fn `PuppetOnGround`
  (returns (OnGround :type Boolean))
  (return (`/Game/Blueprints/Puppet_BP.OnGround` (`/Game/Blueprints/PlanetPawn_BP.Puppet` (`self.PlanetPawn`)))))

(fn `SetPlanetPawn`
  (bind _returnvalue (`GameplayStatics.GetActorOfClass` "/Game/Blueprints/PlanetPawn_BP.PlanetPawn_BP_C"))
  (set `self.PlanetPawn` _returnvalue))

(fn `SetupInput`
  (`EnhancedInputSubsystemInterface.AddMappingContext` (subsystem `EnhancedInputLocalPlayerSubsystem`) "/Game/Input/IMC.IMC" 0 (struct)))

(fn `UserConstructionScript`)