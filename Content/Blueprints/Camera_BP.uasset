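; Camera actor that smoothly follows the puppet held by the level's PlanetPawn_BP.
; On BeginPlay it finds the pawn, and on Tick it reads the pawn's Puppet whenever its own reference is invalid.
; Once the puppet is valid, FollowPuppet lerps the actor each frame from the camera component's world location toward the puppet plus DistanceOffset, using Speed times delta time as alpha.
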(event `self.ReceiveBeginPlay`
  (bind _returnvalue (`GameplayStatics.GetActorOfClass` "/Game/Blueprints/PlanetPawn_BP.PlanetPawn_BP_C"))
  (set `self.PlanetPawn` _returnvalue))

(event `self.ReceiveActorBeginOverlap`
  (params (OtherActor :type "Actor Object Reference")))

(event `self.ReceiveTick`
  (params (DeltaSeconds :type "Float (single-precision)"))
  (if (`KismetSystemLibrary.IsValid` (`self.Puppet`))
    (`self.FollowPuppet` DeltaSeconds)
    (else
      (set `self.Puppet` (`/Game/Blueprints/PlanetPawn_BP.Puppet` (`self.PlanetPawn`))))))

(fn `FollowPuppet`
  (params (Delta :type "Float (double-precision)"))
  (`self.K2_SetActorLocation` (`KismetMathLibrary.VLerp` (`SceneComponent.K2_GetComponentLocation` (`self.CameraComponent`)) (+ (`self.DistanceOffset`) (`self.K2_GetActorLocation` (`self.Puppet`))) (* (`self.Speed`) Delta))))

(fn `UserConstructionScript`)