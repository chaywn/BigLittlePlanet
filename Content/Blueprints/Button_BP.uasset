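; Floor or world button that unlocks the Door_BP whose DoorValue matches its ButtonValue, found by searching all doors at BeginPlay.
; Overlapping the button makes the door translucent and overlap-only, and plays a doorbell sound.
; A positive UnlockDuration gives the button a timer material and schedules LockDoor by timer to restore blocking.
; Tick separately counts down a Timer variable to show the remaining seconds as text.
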(event `self.ReceiveBeginPlay`
  (`self.SetupDoor`))

(event `self.ReceiveTick`
  (params (DeltaSeconds :type "Float (single-precision)"))
  (bind _timer (`self.Timer`))
  (`self.UpdateTimerText`)
  (if (> _timer 0.0)
    (set `self.Timer` (- _timer DeltaSeconds))))

(event `self.Button.OnComponentBeginOverlap`
  (params (OverlappedComponent :type "PrimitiveComponent Object Reference") (OtherActor :type "Actor Object Reference") (OtherComp :type "PrimitiveComponent Object Reference") (OtherBodyIndex :type Integer) (bFromSweep :type Boolean) (SweepResult :type "HitResult Structure (by ref)"))
  (bind _unlockduration (`self.UnlockDuration`))
  (`self.UnlockDoor`)
  (if (> _unlockduration 0.0)
    (`KismetSystemLibrary.K2_SetTimer` null "LockDoor" _unlockduration)))

(fn `LockDoor`
  (bind _door (`self.Door`))
  (bind _door_2 (`/Game/Blueprints/Door_BP.door` _door))
  (if (> (`self.UnlockDuration`) 0.0)
    (`PrimitiveComponent.SetMaterial` _door_2 0 "/Game/Material/M_TimerDoorOpaque.M_TimerDoorOpaque")
    (else
      (`PrimitiveComponent.SetMaterial` _door_2 0 "/Game/Material/M_DoorOpaque.M_DoorOpaque")))
  (`PrimitiveComponent.SetCollisionResponseToAllChannels` _door_2 "ECR_Block")
  (set `/Game/Blueprints/Door_BP.Unlocked` false _door))

(fn `SetupDoor`
  (bind _outactors (`GameplayStatics.GetAllActorsOfClass` "/Game/Blueprints/Door_BP.Door_BP_C"))
  (for _array_element _outactors
    (if (== (`/Game/Blueprints/Door_BP.doorValue` _array_element) (`self.ButtonValue`))
      (bind _output_get (set `self.Door` _array_element))
      (`PrimitiveComponent.SetMaterial` (`/Game/Blueprints/Door_BP.door` _output_get) 0 "/Game/Material/M_TimerDoorOpaque.M_TimerDoorOpaque"))))

(fn `UnlockDoor`
  (bind _door (`self.Door`))
  (bind _unlockduration (`self.UnlockDuration`))
  (bind _door_2 (`/Game/Blueprints/Door_BP.door` _door))
  (if (not (`/Game/Blueprints/Door_BP.Unlocked` _door))
    (if (> _unlockduration 0.0)
      (set `self.Timer` _unlockduration)
      (`PrimitiveComponent.SetMaterial` _door_2 0 "/Game/Material/M_TimerDoorTranslucent.M_TimerDoorTranslucent")
      (else
        (`PrimitiveComponent.SetMaterial` _door_2 0 "/Game/Material/M_DoorTranslucent.M_DoorTranslucent")))
    (`PrimitiveComponent.SetCollisionResponseToAllChannels` _door_2 "ECR_Overlap")
    (set `/Game/Blueprints/Door_BP.Unlocked` true _door)
    (`GameplayStatics.PlaySound2D` "/Game/Audio/doorbell.doorbell" 1.0 1.0 0.0 null null)))

(fn `UpdateTimerText`
  (bind _timertext (`self.TimerText`))
  (bind _timer (`self.Timer`))
  (if (> _timer 0.0)
    (`TextRenderComponent.K2_SetText` _timertext (`KismetTextLibrary.Conv_IntToText` (`KismetMathLibrary.FCeil` _timer)))
    (else
      (`TextRenderComponent.K2_SetText` _timertext (`KismetTextLibrary.Conv_StringToText` " ")))))

(fn `UserConstructionScript`
  (if (> (`self.UnlockDuration`) 0.0)
    (`PrimitiveComponent.SetMaterial` (`self.Button`) 0 "/Game/Material/M_TimerDoorOpaque.M_TimerDoorOpaque")))