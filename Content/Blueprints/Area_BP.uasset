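; Area_BP is a trigger area that shows the level's Goal_BP actor while a tagged object sits inside its box.
; On BeginPlay it hides the goal and clears the HasObject flag.
; Box overlap begin and end events check for the "Object" tag, set HasObject, and show or hide the goal, which is looked up by class each time.
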(event `self.ReceiveBeginPlay`
  (bind _returnvalue (`GameplayStatics.GetActorOfClass` "/Game/Blueprints/Goal_BP.Goal_BP_C"))
  (`self.SetActorHiddenInGame` _returnvalue true)
  (set `self.hasObject` false))

(event `self.Box.OnComponentBeginOverlap`
  (params (OverlappedComponent :type "PrimitiveComponent Object Reference") (OtherActor :type "Actor Object Reference") (OtherComp :type "PrimitiveComponent Object Reference") (OtherBodyIndex :type Integer) (bFromSweep :type Boolean) (SweepResult :type "HitResult Structure (by ref)"))
  (if (`self.ActorHasTag` OtherActor "Object")
    (set `self.hasObject` true)
    (bind _returnvalue (`GameplayStatics.GetActorOfClass` "/Game/Blueprints/Goal_BP.Goal_BP_C"))
    (`self.SetActorHiddenInGame` _returnvalue false)))

(event `self.Box.OnComponentEndOverlap`
  (params (OverlappedComponent :type "PrimitiveComponent Object Reference") (OtherActor :type "Actor Object Reference") (OtherComp :type "PrimitiveComponent Object Reference") (OtherBodyIndex :type Integer))
  (if (`self.ActorHasTag` OtherActor "Object")
    (set `self.hasObject` false)
    (bind _returnvalue (`GameplayStatics.GetActorOfClass` "/Game/Blueprints/Goal_BP.Goal_BP_C"))
    (`self.SetActorHiddenInGame` _returnvalue true)))

(fn `UserConstructionScript`)