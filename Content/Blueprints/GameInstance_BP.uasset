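; GameInstance_BP is the game instance that tracks the current scene and level of a maze game and supplies the matching maze, music and HUD.
; GetLevelMaze returns the current level's maze entry while in the Playing scene, and IncrementLevel wraps back to the first after the last.
; Scene-keyed maps supply HUDs and music, with one reused 2D audio component that only swaps sound when the track differs.
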(fn `Get Scene HUD`
  (returns (HUD :type "UserWidget Class Reference"))
  (return (`BlueprintMapLibrary.Map_Find` (`self.HUDs`) (`self.CurrentScene`))))

(fn `GetLevelMaze`
  (returns (MazePawn :type "/Game/Blueprints/PlanetPawn_BP Class Reference"))
  (if (== (`self.CurrentScene`) "Playing")
    (return (`|GetArrayItem` (`self.MazeBP`) (`self.CurrentLevel`)))
    (else
      (return null))))

(fn `IncrementLevel`
  (bind _result (`/Engine/EditorBlueprintResources/StandardMacros.IncrementInt` (`self.CurrentLevel`))
    (:`  `
      (if (>= _result (`KismetArrayLibrary.Array_Length` (`self.MazeBP`)))
        (set `self.CurrentLevel` 0)))))

(fn `PlayBackgroundAudio`
  (bind _backgroundaudiocomponent (`self.BackgroundAudioComponent`))
  (bind _value (`BlueprintMapLibrary.Map_Find` (`self.Musics`) (`self.CurrentScene`)))
  (if (== (`self.BackgroundAudioComponent`) null)
    (bind _returnvalue (`GameplayStatics.SpawnSound2D` _value 1.0 1.0 0.0 null true false))
    (set `self.BackgroundAudioComponent` _returnvalue)
    (elif (not (== _value (`AudioComponent.Sound` _backgroundaudiocomponent)))
      (`AudioComponent.SetSound` _backgroundaudiocomponent _value))))