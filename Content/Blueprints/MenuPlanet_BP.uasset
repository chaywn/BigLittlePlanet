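; MenuPlanet_BP is a planet actor, apparently for a menu, that manages a Puppet character and tracks whether it stands on a Start area.
; It rotates the Puppet 180 degrees on BeginPlay, and Tick resets it above the Spawn component whenever it has not been rendered recently.
; Overlaps between the Start component and the Puppet's capsule toggle PuppetOnStart and print debug messages.
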(event `self.ReceiveBeginPlay`
  (`parent.ReceiveBeginPlay`)
  (`self.K2_SetActorRotation` (`self.Puppet`) (struct :`Yaw` 180.0) true))

(event `self.ReceiveTick`
  (params (DeltaSeconds :type "Float (single-precision)"))
  (bind _puppet (`self.Puppet`))
  (if (not (`self.WasRecentlyRendered` _puppet 2.0))
    (`self.K2_SetActorTransform` _puppet (`KismetMathLibrary.MakeTransform` (+ (`SceneComponent.K2_GetComponentLocation` (`self.Spawn`)) (0.0 0.0 600.0)) (struct :`Yaw` 180.0)) false false)))

(event `self.Start.OnComponentBeginOverlap`
  (params (OverlappedComponent :type "PrimitiveComponent Object Reference") (OtherActor :type "Actor Object Reference") (OtherComp :type "PrimitiveComponent Object Reference") (OtherBodyIndex :type Integer) (bFromSweep :type Boolean) (SweepResult :type "HitResult Structure (by ref)"))
  (if (== (`Character.CapsuleComponent` (`self.Puppet`)) OtherComp)
    (`KismetSystemLibrary.PrintString` "Overlap")
    (set `self.PuppetOnStart` true)))

(event `self.Start.OnComponentEndOverlap`
  (params (OverlappedComponent :type "PrimitiveComponent Object Reference") (OtherActor :type "Actor Object Reference") (OtherComp :type "PrimitiveComponent Object Reference") (OtherBodyIndex :type Integer))
  (if (== (`Character.CapsuleComponent` (`self.Puppet`)) OtherComp)
    (`KismetSystemLibrary.PrintString` "EndOverlap")
    (set `self.PuppetOnStart` false)))

(fn `UserConstructionScript`)