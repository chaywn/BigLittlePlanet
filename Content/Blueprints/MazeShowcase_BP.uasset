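; MazeShowcase_BP is a showcase actor that rotates itself and spawns Ball_BP actors.
; BeginPlay finds an existing Ball_BP and stores a spawn point raised above it.
; Each Tick adds frame-rate-independent world roll from RotateSpeed until the actor's pitch, rather than roll, nearly equals RotationExtent.
; On a match it updates both speed and extent and spawns another ball at the stored point.
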(event `self.ReceiveBeginPlay`
  (bind _returnvalue (`GameplayStatics.GetActorOfClass` "/Game/Blueprints/Ball_BP.Ball_BP_C"))
  (bind (_returnvalue_x _returnvalue_y _returnvalue_z) (`KismetMathLibrary.BreakVector` (`self.K2_GetActorLocation` _returnvalue)))
  (set `self.SpawnLocation` (`KismetMathLibrary.MakeVector` _returnvalue_x _returnvalue_y (+ _returnvalue_z 500.0))))

(event `self.ReceiveTick`
  (params (DeltaSeconds :type "Float (single-precision)"))
  (bind (_returnvalue_roll _returnvalue_pitch) (`KismetMathLibrary.BreakRotator` (`self.K2_GetActorRotation`)))
  (if (== (`KismetMathLibrary.MakeRotator` 0.0 _returnvalue_pitch) (`KismetMathLibrary.MakeRotator` 0.0 (`self.RotationExtent`)) :`ErrorTolerance` 0.1)
    (`/Engine/EditorBlueprintResources/StandardMacros.NegateFloat` (`self.RotateSpeed`)
      (:`  `
        (`/Engine/EditorBlueprintResources/StandardMacros.NegateFloat` (`self.RotationExtent`)
          (:`  `
            (`|SpawnActorFromClass` "/Game/Blueprints/Ball_BP.Ball_BP_C" (`KismetMathLibrary.MakeTransform` (`self.SpawnLocation`)) "Undefined" "MultiplyWithRoot" null null)))))
    (else
      (`self.K2_AddActorWorldRotation` (`KismetMathLibrary.MakeRotator` (* DeltaSeconds (`self.RotateSpeed`)))))))

(fn `Rotate`)

(fn `UserConstructionScript`)