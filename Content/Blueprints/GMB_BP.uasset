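; GMB_BP is a game mode that sets up each scene and handles level progression in a maze game.
; On construction it starts background audio and takes the default pawn class from GameInstance_BP's current maze.
; BeginPlay adds the scene's HUD, showing the cursor only in the menu.
; NextLevel increments the level, signals completion and returns to the menu when it wraps to zero, and Tick performs the delayed level load.
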(event `self.ReceiveBeginPlay`
  (`self.SetHUD`))

(event `self.ReceiveTick`
  (params (DeltaSeconds :type "Float (single-precision)"))
  ;[1 1 1] Delay before opening level
  (if (`self.OpenLevel`)
    (set `self.OpenLevel` false)
    (`KismetSystemLibrary.Delay` (`self.DelayDuration`))
    (`GameplayStatics.OpenLevel` (`self.NextOpenLevel`))))

(fn `NextLevel`
  (bind _gameinstance (`self.GameInstance`))
  (`/Game/Blueprints/GameInstance_BP.IncrementLevel` _gameinstance)
  (if (== (`/Game/Blueprints/GameInstance_BP.CurrentLevel` _gameinstance) 0)
    (bind _output_get (set `/Game/Blueprints/GameInstance_BP.CurrentScene` "Menu" _gameinstance))
    (set `self.NextOpenLevel` _output_get)
    (set `self.DelayDuration` 5.0)
    (`self.OnGameCompletion`)
    (else
      (set `self.NextOpenLevel` "Maze")))
  (set `self.OpenLevel` true))

(fn `SetHUD`
  (bind _returnvalue (`GameplayStatics.GetPlayerController` 0))
  (bind _gameinstance (`self.GameInstance`))
  (set `PlayerController.bShowMouseCursor` (== (`/Game/Blueprints/GameInstance_BP.CurrentScene` _gameinstance) "Menu") _returnvalue)
  (bind _hud (`/Game/Blueprints/GameInstance_BP.Get Scene HUD` _gameinstance))
  (bind _returnvalue_2 (`|CreateWidget` _hud _returnvalue))
  (bind _output_get (set `self.CurrentHUD` _returnvalue_2))
  (`UserWidget.AddToViewport` _output_get 0))

(fn `SetPawnClass`
  (bind _mazepawn (`/Game/Blueprints/GameInstance_BP.GetLevelMaze` (`self.GameInstance`)))
  (set `self.DefaultPawnClass` _mazepawn))

(fn `UserConstructionScript`
  (bind _asgame_instance_bp (cast `/Game/Blueprints/GameInstance_BP` (`GameplayStatics.GetGameInstance`)))
  (bind _output_get (set `self.GameInstance` _asgame_instance_bp))
  (`/Game/Blueprints/GameInstance_BP.PlayBackgroundAudio` _output_get)
  (`self.SetPawnClass`))