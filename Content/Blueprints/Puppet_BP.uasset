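; Physics-driven Sackboy puppet that moves, jumps, and grips or releases planet objects, bound to player controller events.
; Movement sets capsule velocity and faces the travel direction, while a physical animation profile simulates the mesh's lower bodies.
; Tick checks ground with fallback line traces toward both feet.
; Gripping moves a traced object's constraint from the planet to the puppet and makes it weightless; releasing restores both.
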(event `self.ReceiveBeginPlay`
  (bind _playercontroller (`self.PlayerController`))
  (`self.SetPlanetPawn`)
  (`self.SetPlayerController`)
  (add `/Game/Blueprints/PlayerController_BP.OnPuppetJump` _playercontroller (`|CreateDelegate` :!event `JumpUp`))
  (add `/Game/Blueprints/PlayerController_BP.OnPuppetMoveRight` _playercontroller (`|CreateDelegate` :!event `MoveRight`))
  (add `/Game/Blueprints/PlayerController_BP.OnPuppetMoveForward` _playercontroller (`|CreateDelegate` :!event `MoveForward`))
  (add `/Game/Blueprints/PlayerController_BP.OnGrip` _playercontroller (`|CreateDelegate` :!event `GripObject`))
  (add `/Game/Blueprints/PlayerController_BP.OnRelease` _playercontroller (`|CreateDelegate` :!event `ReleaseObject`))
  (`self.SetPhysicalAnimation`)
  (`PhysicsConstraintComponent.BreakConstraint` (`self.PhysicsConstraint`)))

(event `self.ReceiveTick`
  (params (DeltaSeconds :type "Float (single-precision)"))
  (`self.DetectGround`))

(fn `AddGravityForce`
  (bind _weight (`self.GetWeight`))
  (bind _velocitytoplanet (`self.GetVelocityToPlanet`))
  (`PrimitiveComponent.AddForce` (`self.CapsuleComponent`) (* (`KismetMathLibrary.Normal` _velocitytoplanet) _weight) "None" true))

(fn `DetectGround`
  (bind _returnvalue (`self.K2_GetActorLocation`))
  (bind _sackboy (`self.Sackboy`))
  (bind (_outhit _returnvalue_2) (`KismetSystemLibrary.LineTraceSingle` _returnvalue (+ _returnvalue (* (`self.GetActorUpVector`) (`self.GroundDetectionDistance`))) "TraceTypeQuery1" false (`self.ActorsToIgnoreDetection`)))
  (if _returnvalue_2
    (set `self.OnGround` true :!label _label)
    (else
      (bind (_outhit_2 _returnvalue_3) (`KismetSystemLibrary.LineTraceSingle` _returnvalue (+ (`SceneComponent.GetSocketLocation` _sackboy "RightFoot") (0.0 0.0 -25.0)) "TraceTypeQuery1" false (`self.ActorsToIgnoreDetection`)))
      (if _returnvalue_3
        (goto _label)
        (else
          (bind (_outhit_3 _returnvalue_4) (`KismetSystemLibrary.LineTraceSingle` _returnvalue (+ (`SceneComponent.GetSocketLocation` _sackboy "LeftFoot") (0.0 0.0 -25.0)) "TraceTypeQuery1" false (`self.ActorsToIgnoreDetection`)))
          (if _returnvalue_4
            (goto _label)
            (else
              (set `self.OnGround` false))))))))

(fn `DetectObject`
  (returns (IsDetected :type Boolean))
  (bind _returnvalue (`self.K2_GetActorLocation`))
  (bind _outhit (`KismetSystemLibrary.LineTraceSingle` :`Start` _returnvalue :`End` (+ _returnvalue (+ (* (`self.GetActorForwardVector`) (`self.ObjectDetectionDistance`)) (`self.ObjectDetectionOffset`))) :`TraceChannel` "TraceTypeQuery1" :`DrawDebugType` "ForOneFrame"))
  (bind _asplanet_object_bp (cast `/Game/Blueprints/PlanetObject_BP` (`.HitActor` (`GameplayStatics.BreakHitResult` _outhit)))
    (:`then`
      (set `self.ObjectDetected` _asplanet_object_bp)
      (return true))
    (:`CastFailed`
      (return false))))

(fn `FollowPlanet`
  (bind _capsulecomponent (`self.CapsuleComponent`))
  (bind _capsulecomponent_2 (`self.CapsuleComponent`))
  (bind _velocitytoplanet (`self.GetVelocityToPlanet`))
  ;[1 1 1] Rorate Direction
  (if (>= (.y _velocitytoplanet) 0.0)
    (`SceneComponent.K2_SetRelativeRotation` _capsulecomponent_2 (struct :`Yaw` 90.0) false true)
    (else
      (`SceneComponent.K2_SetRelativeRotation` _capsulecomponent_2 (struct :`Yaw` -90.0) false true)))
  (if (> (`KismetMathLibrary.Abs` (.y _velocitytoplanet)) 40.0)
    (`PrimitiveComponent.SetAllPhysicsLinearVelocity` _capsulecomponent (`KismetMathLibrary.MakeVector` 0.0 (.y _velocitytoplanet)) false)
    (else
      (`PrimitiveComponent.SetAllPhysicsLinearVelocity` _capsulecomponent (0.0 0.0 0.0) true))))

(fn `GetVelocityToPlanet`
  (returns (VelocityToPlanet :type "Vector Structure"))
  (return (- (`SceneComponent.K2_GetComponentLocation` (`/Game/Blueprints/PlanetPawn_BP.Planet` (`self.PlanetPawn`))) (`SceneComponent.K2_GetComponentLocation` (`self.CapsuleComponent`)))))

(fn `GetWeight`
  (returns (Weight :type "Float (double-precision)"))
  (return (* (`PrimitiveComponent.GetMass` (`self.CapsuleComponent`)) (`/Game/Blueprints/PlanetPawn_BP.Gravity` (`self.PlanetPawn`)))))

(fn `GripObject`
  (bind _physicsconstraint (`self.PhysicsConstraint`))
  (bind _objectdetected (`self.ObjectDetected`))
  (bind _object (`/Game/Blueprints/PlanetObject_BP.Object` _objectdetected))
  (`PhysicsConstraintComponent.BreakConstraint` (`/Game/Blueprints/PlanetObject_BP.PhysicsConstraint` _objectdetected))
  (`PhysicsConstraintComponent.SetConstrainedComponents` _physicsconstraint null "None" _object "None")
  (`PhysicsConstraintComponent.SetConstraintReferencePosition` _physicsconstraint "Frame2" (* (`self.ConstraintOffset`) (`SceneComponent.RelativeScale3D` _object)))
  (`PrimitiveComponent.SetMassOverrideInKg` _object "None" 1.0 true)
  (`PrimitiveComponent.SetMassScale` _object "None" 0.0)
  (`PrimitiveComponent.SetEnableGravity` _object false)
  (`KismetArrayLibrary.Array_Insert` (`self.ActorsToIgnoreDetection`) (`self.ObjectDetected`))
  (set `self.IsGripping` true))

(fn `IsEqualDetectedObject`
  (params (Object :type "Actor Object Reference"))
  (returns (IsEqualDetectedObject :type Boolean))
  (bind _asplanet_object_bp (cast `/Game/Blueprints/PlanetObject_BP` Object)
    (:`then`
      (if (`self.IsGripping`)
        (return (== (`self.ObjectDetected`) _asplanet_object_bp))
        (else
          _)))
    (:`CastFailed`
      _))
  (return false))

(fn `JumpUp`
  (`PrimitiveComponent.SetPhysicsLinearVelocity` (`self.CapsuleComponent`) (0.0 0.0 100.0) true "None")
  (set `self.OnGround` false))

(fn `MoveForward`
  (params (VectorX :type "Float (double-precision)"))
  (bind _capsulecomponent (`self.CapsuleComponent`))
  (bind _returnvalue (`PrimitiveComponent.GetPhysicsLinearVelocity` _capsulecomponent "None"))
  (`PrimitiveComponent.SetPhysicsLinearVelocity` _capsulecomponent (`KismetMathLibrary.MakeVector` (* VectorX (`self.Speed`)) (.y _returnvalue) (.z _returnvalue)) false "None")
  ;[1 1 1] Rorate Direction
  (`self.RotateDirection`))

(fn `MoveRight`
  (params (VectorY :type "Float (double-precision)"))
  (bind _capsulecomponent (`self.CapsuleComponent`))
  (bind _returnvalue (`PrimitiveComponent.GetPhysicsLinearVelocity` _capsulecomponent "None"))
  (`PrimitiveComponent.SetPhysicsLinearVelocity` _capsulecomponent (`KismetMathLibrary.MakeVector` (.x _returnvalue) (* VectorY (`self.Speed`)) (.z _returnvalue)) false "None")
  ;[1 1 1] Rorate Direction
  (`self.RotateDirection`))

(fn `ReleaseObject`
  (bind _objectdetected (`self.ObjectDetected`))
  (bind _object (`/Game/Blueprints/PlanetObject_BP.Object` _objectdetected))
  (`PrimitiveComponent.SetMassOverrideInKg` _object "None" 100.0 true)
  (`PrimitiveComponent.SetMassScale` _object "None" 1.0)
  (`PrimitiveComponent.SetEnableGravity` _object true)
  (`PhysicsConstraintComponent.BreakConstraint` (`self.PhysicsConstraint`))
  (`PhysicsConstraintComponent.SetConstrainedComponents` (`/Game/Blueprints/PlanetObject_BP.PhysicsConstraint` _objectdetected) null "None" (`/Game/Blueprints/PlanetPawn_BP.Planet` (`self.PlanetPawn`)) "None")
  (`KismetArrayLibrary.Array_Clear` (`self.ActorsToIgnoreDetection`))
  (set `self.IsGripping` false))

(fn `RotateDirection`
  (bind _returnvalue (`PrimitiveComponent.GetPhysicsLinearVelocity` (`self.CapsuleComponent`) "None"))
  (if (>= (`KismetMathLibrary.VSizeXY` _returnvalue) 10.0)
    (bind (_returnvalue_roll _returnvalue_pitch _returnvalue_yaw) (`KismetMathLibrary.BreakRotator` (`KismetMathLibrary.MakeRotFromX` _returnvalue)))
    (`self.K2_SetActorRotation` (`KismetMathLibrary.MakeRotator` 0.0 0.0 _returnvalue_yaw))))

(fn `SetPhysicalAnimation`
  (bind _sackboy (`self.Sackboy`))
  (bind _physicalanimation (`self.PhysicalAnimation`))
  (bind _bonename (`self.BoneName`))
  (`PhysicalAnimationComponent.SetSkeletalMeshComponent` _physicalanimation _sackboy)
  (`PhysicalAnimationComponent.ApplyPhysicalAnimationProfileBelow` _physicalanimation _bonename "SackProfile" false false)
  (`SkeletalMeshComponent.SetAllBodiesBelowSimulatePhysics` _sackboy _bonename true false))

(fn `SetPlanetPawn`
  (bind _asplanet_pawn_bp (cast `/Game/Blueprints/PlanetPawn_BP` (`GameplayStatics.GetPlayerPawn` 0)))
  (set `self.PlanetPawn` _asplanet_pawn_bp))

(fn `SetPlayerController`
  (bind _asplayer_controller_bp (cast `/Game/Blueprints/PlayerController_BP` (`GameplayStatics.GetPlayerController` 0)))
  (set `self.PlayerController` _asplayer_controller_bp))

(fn `UserConstructionScript`)