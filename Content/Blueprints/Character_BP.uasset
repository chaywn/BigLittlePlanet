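; Character Blueprint for a puppet whose gravity pulls toward the player's planet pawn.
; On BeginPlay it caches the player controller and planet pawn, then binds to the controller's puppet jump event.
; Each tick it sets the movement component's gravity direction to the normalized offset toward that pawn, printing it for debugging.
; An upward-impulse jump function exists, while the physics-based Y-axis follow logic is disconnected.
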(event `self.ReceiveBeginPlay`
  (`self.SetPlayerController`)
  (`self.SetPlanetPawn`)
  (add `/Game/Blueprints/PlayerController_BP.OnPuppetJump` (`self.PlayerController`) (`|CreateDelegate` :!event `Jump_0`)))

(event `self.ReceiveTick`
  (params (DeltaSeconds :type "Float (single-precision)"))
  (`self.SetGravity`))

(fn `FollowPlanet`
  (bind _velocitytoplanet (`self.GetVelocityToPlanet`))
  (if (> (`KismetMathLibrary.Abs` (.y _velocitytoplanet)) 20.0)
    (`PrimitiveComponent.SetAllPhysicsLinearVelocity` (`self.CapsuleComponent`) (`KismetMathLibrary.MakeVector` 0.0 (.y _velocitytoplanet)) false)))

(fn `GetVelocityToPlanet`
  (returns (VelocityToPlanet :type "Vector Structure"))
  (return (- (`self.K2_GetActorLocation` (`self.PlanetPawn`)) (`self.K2_GetActorLocation`))))

(fn `Jump_0`
  (`PrimitiveComponent.AddImpulse` (`self.CapsuleComponent`) (0.0 0.0 100.0) "None" true)
  (`KismetSystemLibrary.PrintString` "Jump2"))

(fn `SetGravity`
  (bind _velocitytoplanet (`self.GetVelocityToPlanet`))
  (bind _returnvalue (`KismetMathLibrary.Normal` _velocitytoplanet))
  (`KismetSystemLibrary.PrintString` (`KismetStringLibrary.Conv_VectorToString` _returnvalue))
  (`CharacterMovementComponent.SetGravityDirection` (`self.CharacterMovement`) _returnvalue))

(fn `SetPlanetPawn`
  (bind _asplanet_pawn_bp (cast `/Game/Blueprints/PlanetPawn_BP` (`GameplayStatics.GetPlayerPawn` 0)))
  (set `self.PlanetPawn` _asplanet_pawn_bp))

(fn `SetPlayerController`
  (bind _asplayer_controller_bp (cast `/Game/Blueprints/PlayerController_BP` (`GameplayStatics.GetPlayerController` 0)))
  (set `self.PlayerController` _asplayer_controller_bp))

(fn `UserConstructionScript`)