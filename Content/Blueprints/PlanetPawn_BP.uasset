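; PlanetPawn_BP is the planet pawn, which rotates in the world in response to the player controller and spawns the puppet character.
; On BeginPlay it binds to PlayerController_BP's OnPlanetRotate, spawns Puppet_BP just above the Spawn component and hides that marker.
; Rotate applies the incoming rotation scaled by RotateSpeed, using the roll sign to check the Left or Right flag in the LockRotation map, which can block that direction.
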(event `self.ReceiveBeginPlay`
  (`self.SetPlayerController`)
  (`self.SpawnPuppet`)
  (`SceneComponent.SetHiddenInGame` (`self.Spawn`) true false))

(fn `Rotate`
  (params (Rotation :type "Rotator Structure"))
  (bind _lockrotation (`self.LockRotation`))
  (bind _returnvalue (> (.roll Rotation) 0.0))
  (if (or (and _returnvalue (not (`BlueprintMapLibrary.Map_Find` _lockrotation "Right"))) (and (not _returnvalue) (not (`BlueprintMapLibrary.Map_Find` _lockrotation "Left"))))
    (`self.K2_AddActorWorldRotation` (* Rotation (`self.RotateSpeed`)))))

(fn `SetPlayerController`
  (bind _asplayer_controller_bp (cast `/Game/Blueprints/PlayerController_BP` (`GameplayStatics.GetPlayerController` 0)))
  (bind _output_get (set `self.PlayerController` _asplayer_controller_bp))
  (add `/Game/Blueprints/PlayerController_BP.OnPlanetRotate` _output_get (`|CreateDelegate` :!event `Rotate`)))

(fn `SpawnPuppet`
  (bind _returnvalue_location (`KismetMathLibrary.BreakTransform` (`SceneComponent.K2_GetComponentToWorld` (`self.Spawn`))))
  (bind _returnvalue (`|SpawnActorFromClass` "/Game/Blueprints/Puppet_BP.Puppet_BP_C" (`KismetMathLibrary.MakeTransform` (+ _returnvalue_location (0.0 0.0 100.0)) (struct :`Yaw` 90.0)) "Undefined" "MultiplyWithRoot" null null))
  (set `self.Puppet` _returnvalue))

(fn `UserConstructionScript`)